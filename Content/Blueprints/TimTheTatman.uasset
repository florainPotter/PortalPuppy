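; Player character with cursor-aimed facing, axis movement, jump, a timed forward charge, and a box-pushing mechanic.
; Pressing E while overlapping and facing a PushabelBox lerps the character to the active side via timelines and locks input to pushing with W.
; A looping timer keeps the box ahead of the character until Q releases it.
; A per-tick sphere trace halts movement when the push is blocked.
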(event `self.ReceiveBeginPlay`
  (`ActorComponent.Activate` (`self.Camera`) false)
  (bind _outactors (`GameplayStatics.GetAllActorsOfClass` "/Game/Blueprints/PushabelBox.PushabelBox_C"))
  (set `self.boxes` _outactors))

(event `InputAxis|updown`
  (params (AxisValue :type "Float (single-precision)"))
  (bind _pushing (`self.Pushing`))
  ;[1 1 1] base movement input
  (if (or _pushing (`self.charging`))
    (if _pushing
      (`self.AddMovementInput` (`self.pushDirection`) (`self.pushVelocity`)))
    (else
      (`self.AddMovementInput` (1.0 0.0 0.0) AxisValue))))

(event `InputAxis|leftright`
  (params (AxisValue :type "Float (single-precision)"))
  ;[1 1 1] base movement input
  (if (not (or (`self.Pushing`) (`self.charging`)))
    (`self.AddMovementInput` (0.0 1.0 0.0) AxisValue)))

(event `MoveBox`
  (bind _returnvalue (`GameplayStatics.GetPlayerCharacter` 0))
  ;[1 1 1] update box location acording to pawn
  (`self.K2_SetActorLocation` null (`KismetMathLibrary.VInterpTo` (`self.K2_GetActorLocation`) (- (+ (* (`self.GetActorForwardVector` _returnvalue) 150.0) (`self.K2_GetActorLocation` _returnvalue)) (0.0 0.0 -20.0)) (`GameplayStatics.GetWorldDeltaSeconds`) 100.0) false false)
  (set `CharacterMovementComponent.MaxWalkSpeed` 120.0 (`self.CharacterMovement`))
  (if (`self.Qdown`)
    _))

(event `self.ReceiveTick`
  (params (DeltaSeconds :type "Float (single-precision)"))
  (bind _returnvalue (`GameplayStatics.GetPlayerController` 0))
  (bind (_returnvalue_x _returnvalue_y _returnvalue_z) (`KismetMathLibrary.BreakVector` (`self.K2_GetActorLocation`)))
  (bind (_returnvalue_x_2 _returnvalue_y_2 _returnvalue_z_2) (`KismetMathLibrary.BreakVector` (`KismetMathLibrary.GetForwardVector` (`self.K2_GetActorRotation`))))
  (bind _returnvalue_2 (`KismetMathLibrary.MakeVector` _returnvalue_x _returnvalue_y (- _returnvalue_z 0.0)))
  (`|ExecutionSequence`
    (:`then_0`
      ;[1 1 1] lookaround
      (if (not (or (`self.charging`) (`self.Pushing`)))
        (`Controller.SetControlRotation` _returnvalue (`KismetMathLibrary.FindLookAtRotation` (`self.K2_GetActorLocation` (`Controller.K2_GetPawn` _returnvalue)) (`.Location` (`GameplayStatics.BreakHitResult` (`PlayerController.GetHitResultUnderCursorByChannel` _returnvalue "TraceTypeQuery1" true)))))))
    (:`then_1`
      ;[1 1 1] pushing collision
      (bind (_outhit _returnvalue_3) (`KismetSystemLibrary.SphereTraceSingle` _returnvalue_2 (+ _returnvalue_2 (`KismetMathLibrary.MakeVector` (* _returnvalue_x_2 230.0) (* _returnvalue_y_2 230.0) (- _returnvalue_z_2 0.0))) 50.0 "TraceTypeQuery1" false (`self.boxes`) "ForOneFrame"))
      (set `self.colliding` (and _returnvalue_3 (`self.Pushing`) (`GameplayStatics.BreakHitResult` _outhit))))))

(event `InputAction|Jump`
  (params (Key :type "Key Structure"))
  ;[1 1 1] base movement input
  (:`Pressed`
    (if (not (or (`self.Pushing`) (`self.charging`)))
      (`self.Jump`)))
  (:`Released`
    (`self.StopJumping`)))

(event `charge`
  (bind _charactermovement (`self.CharacterMovement`))
  (set `self.charging` true)
  (set `self.chargeDirection` (`self.GetActorForwardVector`))
  (set `CharacterMovementComponent.MaxWalkSpeed` 1000.0 _charactermovement)
  (`Timeline|shargeTime` :!via `PlayFromStart`
    (:`Update`
      (`self.AddMovementInput` (`self.chargeDirection`)))
    (:`Finished`
      (set `CharacterMovementComponent.MaxWalkSpeed` 600.0 _charactermovement)
      (set `self.charging` false))))

(event `Key|E`
  (params (Key :type "Key Structure"))
  ;[1 1 1] push box
  (:`Pressed`
    (set `self.Edown` true))
  (:`Released`
    (set `self.Edown` false)))

(event `Key|W`
  (params (Key :type "Key Structure"))
  ;[1 1 1] push box
  (:`Pressed`
    (set `self.pushVelocity` 1.0))
  (:`Released`
    (set `self.pushVelocity` 0.0)))

(event `Key|Q`
  (params (Key :type "Key Structure"))
  ;[1 1 1] push box
  (:`Pressed`
    (set `self.Qdown` true))
  (:`Released`
    (set `self.Qdown` false)))

(event `Key|S`
  (params (Key :type "Key Structure"))
  ;[1 1 1] push box
)

(event `Key|E`
  (params (Key :type "Key Structure"))
  (bind _returnvalue (`GameplayStatics.GetPlayerCharacter` 0))
  (bind _returnvalue_2 (`GameplayStatics.GetPlayerCharacter` 0))
  (bind _returnvalue_3 (`GameplayStatics.GetPlayerCharacter` 0))
  (bind _returnvalue_4 (`GameplayStatics.GetPlayerCharacter` 0))
  ;[1 1 1] push box
  (:`Pressed`
    (`/Engine/EditorBlueprintResources/StandardMacros.Gate` true :!label _label
      (:`Exit`
        (bind _accepted (`self.IsAngleAcceptable` (- (`self.K2_GetActorLocation` (stale `self.ReceiveActorBeginOverlap` _aspushabel_box)) (`self.K2_GetActorLocation`)) (`self.GetActorForwardVector`) 10.0))
        (if _accepted
          (set `CharacterMovementComponent.MaxWalkSpeed` 120.0 (`self.CharacterMovement`))
          (`|ExecutionSequence`
            (:`then_0`
              ;;[1 1 1] lerp character to side of box (side 0)
              (if (`/Game/Blueprints/PushabelBox.side0` (stale `self.ReceiveActorBeginOverlap` _aspushabel_box))
                (set `self.Pushing` true)
                (bind (_direction _alpha) (`Timeline|Transition0` :!via `PlayFromStart`)
                  (:`Update`
                    (`self.K2_SetActorLocationAndRotation` _returnvalue_2 (`KismetMathLibrary.VLerp` (`self.K2_GetActorLocation` _returnvalue_2) (`SceneComponent.K2_GetComponentLocation` (`/Game/Blueprints/PushabelBox.TPpoint0` (stale `self.ReceiveActorBeginOverlap` _aspushabel_box))) _alpha) (`KismetMathLibrary.RLerp` (`self.K2_GetActorRotation` _returnvalue_2) (`SceneComponent.K2_GetComponentRotation` (`/Game/Blueprints/PushabelBox.arrow0` (stale `self.ReceiveActorBeginOverlap` _aspushabel_box))) _alpha true) false false))
                  (:`Finished`
                    (bind _returnvalue_5 (`KismetSystemLibrary.K2_SetTimerDelegate` (delegate `updateboxpos`) 0.005 true :!label _label_2))))))
            (:`then_1`
              ;;[1 1 1] lerp character to side of box (side 1)
              (if (`/Game/Blueprints/PushabelBox.side1` (stale `self.ReceiveActorBeginOverlap` _aspushabel_box))
                (set `self.Pushing` true)
                (bind (_direction_2 _alpha_2) (`Timeline|Transition1` :!via `PlayFromStart`)
                  (:`Update`
                    (`self.K2_SetActorLocationAndRotation` _returnvalue_4 (`KismetMathLibrary.VLerp` (`self.K2_GetActorLocation` _returnvalue_4) (`SceneComponent.K2_GetComponentLocation` (`/Game/Blueprints/PushabelBox.TPpoint1` (stale `self.ReceiveActorBeginOverlap` _aspushabel_box))) _alpha_2) (`KismetMathLibrary.RLerp` (`self.K2_GetActorRotation` _returnvalue_4) (`SceneComponent.K2_GetComponentRotation` (`/Game/Blueprints/PushabelBox.arrow1` (stale `self.ReceiveActorBeginOverlap` _aspushabel_box))) _alpha_2 true) false false))
                  (:`Finished`
                    (goto _label_2)))))
            (:`then_2`
              ;;[1 1 1] lerp character to side of box (side 2)
              (if (`/Game/Blueprints/PushabelBox.side2` (stale `self.ReceiveActorBeginOverlap` _aspushabel_box))
                (set `self.Pushing` true)
                (bind (_direction_3 _alpha_3) (`Timeline|Transition2` :!via `PlayFromStart`)
                  (:`Update`
                    (`self.K2_SetActorLocationAndRotation` _returnvalue_3 (`KismetMathLibrary.VLerp` (`self.K2_GetActorLocation` _returnvalue_3) (`SceneComponent.K2_GetComponentLocation` (`/Game/Blueprints/PushabelBox.TPpoint2` (stale `self.ReceiveActorBeginOverlap` _aspushabel_box))) _alpha_3) (`KismetMathLibrary.RLerp` (`self.K2_GetActorRotation` _returnvalue_3) (`SceneComponent.K2_GetComponentRotation` (`/Game/Blueprints/PushabelBox.arrow2` (stale `self.ReceiveActorBeginOverlap` _aspushabel_box))) _alpha_3 true) false false))
                  (:`Finished`
                    (goto _label_2)))))
            (:`then_3`
              ;;[1 1 1] lerp character to side of box (side 3)
              (if (`/Game/Blueprints/PushabelBox.side3` (stale `self.ReceiveActorBeginOverlap` _aspushabel_box))
                (set `self.Pushing` true)
                (bind (_direction_4 _alpha_4) (`Timeline|Transition3` :!via `PlayFromStart`)
                  (:`Update`
                    (`self.K2_SetActorLocationAndRotation` _returnvalue (`KismetMathLibrary.VLerp` (`self.K2_GetActorLocation` _returnvalue) (`SceneComponent.K2_GetComponentLocation` (`/Game/Blueprints/PushabelBox.TPpoint3` (stale `self.ReceiveActorBeginOverlap` _aspushabel_box))) _alpha_4) (`KismetMathLibrary.RLerp` (`self.K2_GetActorRotation` _returnvalue) (`SceneComponent.K2_GetComponentRotation` (`/Game/Blueprints/PushabelBox.arrow3` (stale `self.ReceiveActorBeginOverlap` _aspushabel_box))) _alpha_4 true) false false))
                  (:`Finished`
                    (goto _label_2))))))))))
  (:`Released`
    (goto _label :!via `Close`)))

(event `self.ReceiveActorBeginOverlap`
  (params (OtherActor :type "Actor Object Reference"))
  ;[1 1 1] push box
  (bind _aspushabel_box (cast `/Game/Blueprints/PushabelBox` OtherActor))
  (goto _label :!via `Open`))

(event `self.ReceiveActorEndOverlap`
  (params (OtherActor :type "Actor Object Reference"))
  ;[1 1 1] push box
  (cast `/Game/Blueprints/PushabelBox` OtherActor)
  (goto _label :!via `Close`))

(event `updateboxpos`
  (bind _returnvalue (`GameplayStatics.GetPlayerCharacter` 0))
  (bind _charactermovement (`self.CharacterMovement`))
  ;[1 1 1] push box
  (if (`self.colliding`)
    (`CharacterMovementComponent.DisableMovement` (`self.CharacterMovement`))
    (else
      (`self.K2_SetActorLocation` (stale `self.ReceiveActorBeginOverlap` _aspushabel_box) (- (+ (`self.K2_GetActorLocation` _returnvalue) (* (`self.GetActorForwardVector` _returnvalue) 170.0)) (0.0 0.0 -20.0)) false false)))
  (if (`self.Qdown`)
    (`KismetSystemLibrary.K2_ClearAndInvalidateTimerHandle` (stale `Key|E` _returnvalue_5))
    (set `CharacterMovementComponent.MaxWalkSpeed` 600.0 _charactermovement)
    (`CharacterMovementComponent.SetMovementMode` _charactermovement "MOVE_Walking" 0)
    (set `self.Pushing` false)))

(fn `IsAngleAcceptable`
  (params (start :type "Vector Structure") (target :type "Vector Structure") (maxAngle :type "Float (double-precision)"))
  (returns (accepted :type Boolean))
  (locals (absRotation :type "Float (double-precision)"))
  (return (<= (`KismetMathLibrary.DegAcos` (`KismetMathLibrary.Dot_VectorVector` (`KismetMathLibrary.Normal` start) (`KismetMathLibrary.Normal` target))) maxAngle)))

(fn `UserConstructionScript`)