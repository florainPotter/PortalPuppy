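; Pushable box actor that tells the TimTheTatman character which direction to push based on the side it stands at.
; Four side colliders each set the character's PushDirection to a fixed positive or negative X or Y axis vector on begin overlap.
; Each collider also toggles its own Side flag on begin and end overlap, while the box contains no movement logic itself.
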(event `self.PushCollider0.OnComponentBeginOverlap`
  (params (OverlappedComponent :type "PrimitiveComponent Object Reference") (OtherActor :type "Actor Object Reference") (OtherComp :type "PrimitiveComponent Object Reference") (OtherBodyIndex :type Integer) (bFromSweep :type Boolean) (SweepResult :type "HitResult Structure (by ref)"))
  (bind _astim_the_tatman (cast `/Game/Blueprints/TimTheTatman` OtherActor))
  (set `/Game/Blueprints/TimTheTatman.pushDirection` (1.0 0.0 0.0) _astim_the_tatman)
  (set `self.side0` true))

(event `self.PushCollider0.OnComponentEndOverlap`
  (params (OverlappedComponent :type "PrimitiveComponent Object Reference") (OtherActor :type "Actor Object Reference") (OtherComp :type "PrimitiveComponent Object Reference") (OtherBodyIndex :type Integer))
  (cast `/Game/Blueprints/TimTheTatman` OtherActor)
  (set `self.side0` false))

(event `self.PushCollider1.OnComponentBeginOverlap`
  (params (OverlappedComponent :type "PrimitiveComponent Object Reference") (OtherActor :type "Actor Object Reference") (OtherComp :type "PrimitiveComponent Object Reference") (OtherBodyIndex :type Integer) (bFromSweep :type Boolean) (SweepResult :type "HitResult Structure (by ref)"))
  (bind _astim_the_tatman (cast `/Game/Blueprints/TimTheTatman` OtherActor))
  (set `/Game/Blueprints/TimTheTatman.pushDirection` (-1.0 0.0 0.0) _astim_the_tatman)
  (set `self.side1` true))

(event `self.PushCollider1.OnComponentEndOverlap`
  (params (OverlappedComponent :type "PrimitiveComponent Object Reference") (OtherActor :type "Actor Object Reference") (OtherComp :type "PrimitiveComponent Object Reference") (OtherBodyIndex :type Integer))
  (cast `/Game/Blueprints/TimTheTatman` OtherActor)
  (set `self.side1` false))

(event `self.PushCollider2.OnComponentBeginOverlap`
  (params (OverlappedComponent :type "PrimitiveComponent Object Reference") (OtherActor :type "Actor Object Reference") (OtherComp :type "PrimitiveComponent Object Reference") (OtherBodyIndex :type Integer) (bFromSweep :type Boolean) (SweepResult :type "HitResult Structure (by ref)"))
  (bind _astim_the_tatman (cast `/Game/Blueprints/TimTheTatman` OtherActor))
  (set `/Game/Blueprints/TimTheTatman.pushDirection` (0.0 1.0 0.0) _astim_the_tatman)
  (set `self.side2` true))

(event `self.PushCollider2.OnComponentEndOverlap`
  (params (OverlappedComponent :type "PrimitiveComponent Object Reference") (OtherActor :type "Actor Object Reference") (OtherComp :type "PrimitiveComponent Object Reference") (OtherBodyIndex :type Integer))
  (cast `/Game/Blueprints/TimTheTatman` OtherActor)
  (set `self.side2` false))

(event `self.PushCollider3.OnComponentBeginOverlap`
  (params (OverlappedComponent :type "PrimitiveComponent Object Reference") (OtherActor :type "Actor Object Reference") (OtherComp :type "PrimitiveComponent Object Reference") (OtherBodyIndex :type Integer) (bFromSweep :type Boolean) (SweepResult :type "HitResult Structure (by ref)"))
  (bind _astim_the_tatman (cast `/Game/Blueprints/TimTheTatman` OtherActor))
  (set `/Game/Blueprints/TimTheTatman.pushDirection` (0.0 -1.0 0.0) _astim_the_tatman)
  (set `self.side3` true))

(event `self.PushCollider3.OnComponentEndOverlap`
  (params (OverlappedComponent :type "PrimitiveComponent Object Reference") (OtherActor :type "Actor Object Reference") (OtherComp :type "PrimitiveComponent Object Reference") (OtherBodyIndex :type Integer))
  (cast `/Game/Blueprints/TimTheTatman` OtherActor)
  (set `self.side3` false))

(fn `UserConstructionScript`)