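; Destructible wall actor that the TimTheTatman player can break by pressing Left Shift while standing next to it.
; Box overlaps with the player toggle an in-range flag and enable or disable the wall's own input.
; Left Shift applies radius damage to the DestructibleComponent at the actor's location, then calls Charge on the player with the wall as argument.
; The player reference is found at BeginPlay and can be replaced through setplayer.
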(event `self.ReceiveBeginPlay`
  (bind _outactors (`GameplayStatics.GetAllActorsOfClass` "/Game/Blueprints/TimTheTatman.TimTheTatman_C"))
  (set `self.TimTheTatman` (`|GetArrayItem` _outactors)))

(event `set player`
  (params (player :type "/Game/Blueprints/TimTheTatman Object Reference"))
  (set `self.TimTheTatman` player))

(event `self.Box.OnComponentBeginOverlap`
  (params (OverlappedComponent :type "PrimitiveComponent Object Reference") (OtherActor :type "Actor Object Reference") (OtherComp :type "PrimitiveComponent Object Reference") (OtherBodyIndex :type Integer) (bFromSweep :type Boolean) (SweepResult :type "HitResult Structure (by ref)"))
  (cast `/Game/Blueprints/TimTheTatman` OtherActor)
  (set `self.inRange` true)
  (`self.EnableInput` (`GameplayStatics.GetPlayerController` 0)))

(event `self.Box.OnComponentEndOverlap`
  (params (OverlappedComponent :type "PrimitiveComponent Object Reference") (OtherActor :type "Actor Object Reference") (OtherComp :type "PrimitiveComponent Object Reference") (OtherBodyIndex :type Integer))
  (cast `/Game/Blueprints/TimTheTatman` OtherActor)
  (set `self.inRange` false)
  (`self.DisableInput` (`GameplayStatics.GetPlayerController` 0)))

(event `Key|LeftShift`
  (params (Key :type "Key Structure"))
  (:`Pressed`
    (if (`self.inRange`)
      (`DestructibleComponent.ApplyRadiusDamage` (`self.DestructibleComponent`) 30.0 (`self.K2_GetActorLocation`) 1.0 1.0 false)
      (`/Game/Blueprints/TimTheTatman.charge` (`self.TimTheTatman`) self))))

(fn `UserConstructionScript`)